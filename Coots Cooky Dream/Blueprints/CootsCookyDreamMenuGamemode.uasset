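; Game mode for Coots Cooky Dream, named for the menu, that tracks score, level time, checkpoints and player respawns.
; BeginPlay caches collectables, player and checkpoints, picks the level-start checkpoint, and starts a looping timer.
; Failure spawns a new PlayerCoots at the current checkpoint, transfers possession and physics state, and destroys the old pawn.
; Pickups raise the score; checkpoints record section times by their index in the GetAllActorsOfClass list.
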(event `PlayerFail`
  (bind _playercontroller (`self.PlayerController`))
  (bind _returnvalue (`|SpawnActorFromClass` "/Game/ThirdPerson/Blueprints/PlayerCoots.PlayerCoots_C" (`KismetMathLibrary.MakeTransform` (`self.K2_GetActorLocation` (`self.CurrentCheckPoint`))) "Undefined" "OverrideRootScale" null null))
  (`PrimitiveComponent.SetSimulatePhysics` (`Character.CapsuleComponent` _returnvalue) (`SceneComponent.IsSimulatingPhysics` (`Character.CapsuleComponent` (`self.Player`)) "None"))
  (`Controller.UnPossess` _playercontroller)
  (`Controller.Possess` _playercontroller _returnvalue)
  (`self.K2_DestroyActor` (`self.Player`))
  (set `self.Player` _returnvalue))

(event `self.ReceiveBeginPlay`
  (bind _outactors (`GameplayStatics.GetAllActorsOfClass` "/Game/ThirdPerson/Blueprints/CollectablePickup.CollectablePickup_C"))
  (set `self.Collectable List` _outactors)
  (bind _outactors_2 (`GameplayStatics.GetAllActorsOfClass` "/Game/ThirdPerson/Blueprints/PlayerCoots.PlayerCoots_C"))
  (for _array_element _outactors_2
    (bind _output_get (set `self.Player` _array_element))
    (set `self.PlayerController` (`Pawn.GetController` _output_get)))
  (bind _outactors_3 (`GameplayStatics.GetAllActorsOfClass` "/Game/ThirdPerson/Blueprints/CheckPoint.CheckPoint_C"))
  (bind _output_get_2 (set `self.CheckPointList` _outactors_3))
  (for _array_element_2 _output_get_2
    (if (`/Game/ThirdPerson/Blueprints/CheckPoint.IsLevelStart` _array_element_2)
      (set `self.CurrentCheckPoint` _array_element_2)))
  (`KismetSystemLibrary.K2_SetTimer` null "LevelTimer" (`self.LevelTimerTickRate`) true))

(event `PlayerCollectedPu`
  (params (CollectedPu :type "/Game/ThirdPerson/Blueprints/CollectablePickup Object Reference"))
  (`KismetArrayLibrary.Array_RemoveItem` (`self.Collectable List`) CollectedPu)
  (`self.K2_DestroyActor` CollectedPu)
  (`/Engine/EditorBlueprintResources/StandardMacros.IncrementInt` (`self.LevelScore`)))

(fn `CheckPointReached`
  (params (InPoint :type "/Game/ThirdPerson/Blueprints/CheckPoint Object Reference"))
  (bind _output_get (set `self.CurrentCheckPoint` InPoint))
  (switch `int` (`KismetArrayLibrary.Array_Find` (`self.CheckPointList`) _output_get)
    (:`1`
      (set `self.Section1Time` (`self.LevelTime`)))
    (:`2`
      (set `self.Section2Time` (`self.LevelTime`)))
    (:`3`
      (set `self.Section3Time` (`self.LevelTime`)))))

(fn `LevelTimer`
  (set `self.LevelTime` (+ (`self.LevelTime`) (`self.LevelTimerTickRate`))))

(fn `UserConstructionScript`)