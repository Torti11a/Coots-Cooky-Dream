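; Game mode for Coots Cooky Dream that runs level score, timing, pausing and player respawning.
; BeginPlay caches pickups, player and checkpoints, then starts a looping timer; collected pickups raise the score.
; Failure replaces the pawn at the current checkpoint, set only from the level-start one, keeping its UI.
; CheckPointReached parses the checkpoint name's last character to record section times, with the third opening a map chosen by level number.
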(event `PlayerFail`
  (bind _playercontroller (`self.PlayerController`))
  (bind _returnvalue (`|SpawnActorFromClass` "/Game/ThirdPerson/Blueprints/PlayerCoots.PlayerCoots_C" (`KismetMathLibrary.MakeTransform` (`self.K2_GetActorLocation` (`self.CurrentCheckPoint`))) "Undefined" "OverrideRootScale" null null))
  (set `/Game/ThirdPerson/Blueprints/PlayerCoots.PlayerUI` (`/Game/ThirdPerson/Blueprints/PlayerCoots.PlayerUI` (`self.Player`)) _returnvalue)
  (`PrimitiveComponent.SetSimulatePhysics` (`Character.CapsuleComponent` _returnvalue) true)
  (`Controller.UnPossess` _playercontroller)
  (`Controller.Possess` _playercontroller _returnvalue)
  (`self.K2_DestroyActor` (`self.Player`))
  (set `self.Player` _returnvalue))

(event `self.ReceiveBeginPlay`
  (bind _outactors (`GameplayStatics.GetAllActorsOfClass` "/Game/ThirdPerson/Blueprints/CollectablePickup.CollectablePickup_C"))
  (set `self.Collectable List` _outactors)
  (bind _outactors_2 (`GameplayStatics.GetAllActorsOfClass` "/Game/ThirdPerson/Blueprints/PlayerCoots.PlayerCoots_C"))
  (for _array_element _outactors_2
    (bind _output_get (set `self.Player` _array_element))
    (set `self.PlayerController` (`Pawn.GetController` _output_get)))
  (bind _outactors_3 (`GameplayStatics.GetAllActorsOfClass` "/Game/ThirdPerson/Blueprints/CheckPoint.CheckPoint_C"))
  (bind _output_get_2 (set `self.CheckPointList` _outactors_3))
  (for _array_element_2 _output_get_2
    (if (`/Game/ThirdPerson/Blueprints/CheckPoint.IsLevelStart` _array_element_2)
      (set `self.CurrentCheckPoint` _array_element_2)))
  (`KismetSystemLibrary.K2_SetTimer` null "LevelTimer" (`self.LevelTimerTickRate`) true))

(event `PlayerCollectedPu`
  (params (CollectedPu :type "/Game/ThirdPerson/Blueprints/CollectablePickup Object Reference"))
  (`KismetArrayLibrary.Array_RemoveItem` (`self.Collectable List`) CollectedPu)
  (`self.K2_DestroyActor` CollectedPu)
  (`/Engine/EditorBlueprintResources/StandardMacros.IncrementInt` (`self.LevelScore`)))

(event `Pause timer`
  (params (`Pause?` :type Boolean))
  (if `Pause?`
    (`KismetSystemLibrary.K2_SetTimer` null "LevelTimer" 0.0 true)
    (else
      (`KismetSystemLibrary.K2_SetTimer` null "LevelTimer" (`self.LevelTimerTickRate`) true))))

(event `Pause`
  (bind _returnvalue (`GameplayStatics.GetPlayerController` 0))
  (bind _player (`self.Player`))
  (bind _playerui (`/Game/ThirdPerson/Blueprints/PlayerCoots.PlayerUI` _player))
  (`GameplayStatics.SetGamePaused` true)
  (set `/Game/ThirdPerson/Blueprints/PlayerCoots.CanMove` false _player)
  (`/Engine/EditorBlueprintResources/StandardMacros.IsValid` _playerui
    (:`Is Valid`
      (`Widget.SetVisibility` (`/Game/ThirdPerson/UI/PlayerUI.VerticalBox_48` _playerui) "Visible")
      (`WidgetBlueprintLibrary.SetInputMode_GameAndUIEx` _returnvalue _playerui "DoNotLock" false true)
      (set `PlayerController.bShowMouseCursor` true _returnvalue)
      (`self.Pause timer` true))))

(event `Resume`
  (bind _returnvalue (`GameplayStatics.GetPlayerController` 0))
  (bind _player (`self.Player`))
  (bind _playerui (`/Game/ThirdPerson/Blueprints/PlayerCoots.PlayerUI` _player))
  (`GameplayStatics.SetGamePaused` false)
  (set `/Game/ThirdPerson/Blueprints/PlayerCoots.CanMove` true _player)
  (`/Engine/EditorBlueprintResources/StandardMacros.IsValid` _playerui
    (:`Is Valid`
      (`Widget.SetVisibility` (`/Game/ThirdPerson/UI/PlayerUI.VerticalBox_48` _playerui) "Hidden")
      (`WidgetBlueprintLibrary.SetInputMode_GameOnly` _returnvalue true)
      (set `PlayerController.bShowMouseCursor` false _returnvalue)
      (`self.Pause timer` false))))

(fn `CheckPointReached`
  (params (InPoint :type "/Game/ThirdPerson/Blueprints/CheckPoint Object Reference"))
  (bind _returnvalue (`KismetSystemLibrary.GetDisplayName` InPoint))
  (switch `int` (`KismetStringLibrary.Conv_StringToInt` (`|GetArrayItem` (`KismetStringLibrary.GetCharacterArrayFromString` _returnvalue) (- (`KismetStringLibrary.Len` _returnvalue) 1)))
    (:`1`
      (set `self.Section1Time` (`self.LevelTime`)))
    (:`2`
      (set `self.Section2Time` (`self.LevelTime`)))
    (:`3`
      (set `self.Section3Time` (`self.LevelTime`))
      (switch `int` (+ (`self.Level`) 1)
        (:`0`
          (bind (_boutsuccess _returnvalue_2) (`LevelStreamingDynamic.LoadLevelInstanceBySoftObjectPtr` "/Game/ThirdPerson/Maps/ThirdPersonMap_2.ThirdPersonMap_2" (0.0 0.0 0.0) (struct) "" null))
          (if _boutsuccess
            (`GameplayStatics.OpenLevelBySoftObjectPtr` (`LevelStreaming.WorldAsset` _returnvalue_2))
            (else
              (`KismetSystemLibrary.PrintString` "No level loaded"))))
        (:`1`
          (bind (_boutsuccess_2 _returnvalue_3) (`LevelStreamingDynamic.LoadLevelInstanceBySoftObjectPtr` "/Game/ThirdPerson/Maps/ThirdPersonMap_2.ThirdPersonMap_2" (0.0 0.0 0.0) (struct) "" null))
          (if _boutsuccess_2
            (`GameplayStatics.OpenLevelBySoftObjectPtr` "/Game/ThirdPerson/Maps/ThirdPersonMap_2.ThirdPersonMap_2")
            (else
              (`KismetSystemLibrary.PrintString` "No level loaded"))))
        (:`2`
          (bind (_boutsuccess_3 _returnvalue_4) (`LevelStreamingDynamic.LoadLevelInstanceBySoftObjectPtr` "/Game/ThirdPerson/Maps/ThirdPersonMap_3.ThirdPersonMap_3" (0.0 0.0 0.0) (struct) "" null))
          (if _boutsuccess_3
            (`GameplayStatics.OpenLevelBySoftObjectPtr` "/Game/ThirdPerson/Maps/ThirdPersonMap_3.ThirdPersonMap_3")
            (else
              (`KismetSystemLibrary.PrintString` "No level loaded"))))))))

(fn `LevelTimer`
  (set `self.LevelTime` (+ (`self.LevelTime`) (`self.LevelTimerTickRate`))))

(fn `UserConstructionScript`)